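; Base Blueprint for interactable items, carrying item info and a widget component that holds an interaction prompt.
; On BeginPlay it casts the component's user widget to Interaction_Widget, fills in the item name from ItemInfo and a fixed "[E] Interact" label, then hides it.
; The construction script only calls its parent, and no logic for showing the prompt or handling interaction appears here.
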(event `self.ReceiveBeginPlay`
  (bind _asinteraction_widget (cast `/Game/++Widgets/Interaction_Widget` (`WidgetComponent.GetUserWidgetObject` (`self.Widget`))))
  (`TextBlock.SetText` (`/Game/++Widgets/Interaction_Widget.Name` _asinteraction_widget) (`.ItemName_9_E0AA28F44657592496C412B319906FD0` (break `/Game/++Structures/Item_Info` (`self.ItemInfo`))))
  (`TextBlock.SetText` (`/Game/++Widgets/Interaction_Widget.InteractText` _asinteraction_widget) "[E] Interact")
  (`Widget.SetVisibility` _asinteraction_widget "Hidden"))

(fn `UserConstructionScript`
  (`parent.UserConstructionScript`))