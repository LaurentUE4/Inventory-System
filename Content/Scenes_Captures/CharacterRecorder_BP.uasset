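; CharacterRecorder_BP is a stand-in character in Scenes_Captures that displays equipped items on its skeletal mesh, likely for a scene-capture preview.
; On BeginPlay it passes itself to PlayerChar_BP; EquipItem and UnequipItem events forward to AttachItem and UnattachItem.
; AttachItem switches on equip slot, replaces that slot's actor and snaps the new one, collision disabled, to the socket named in its item info; Arms spawns two pieces.
; UnattachItem destroys the slot's actors.
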(event `self.ReceiveBeginPlay`
  (bind _asplayer_char_bp (cast `/Game/Player_BP/PlayerChar_BP` (`GameplayStatics.GetPlayerCharacter` 0)))
  (message `/Game/++Interfaces/RecorderComm_BPI.PassReference` _asplayer_char_bp self))

(event `/Game/++Interfaces/RecorderComm_BPI.EquipItem`
  (params (ItemInfo :type "/Game/++Structures/Item_Info Structure"))
  (`self.AttachItem` ItemInfo))

(event `/Game/++Interfaces/RecorderComm_BPI.UnequipItem`
  (params (ItemInfo :type "/Game/++Structures/Item_Info Structure"))
  (`self.UnattachItem` ItemInfo))

(fn `AttachItem`
  (params (ItemInfo :type "/Game/++Structures/Item_Info Structure"))
  (bind ((`ItemClass_63_425D6E44495EC74761E86F81359D3E1B` _itemclass) (`ItemEquipSlot_21_E736EAB8438F0A6E85940E8CBD1C71C5` _itemequipslot)) (break `/Game/++Structures/Item_Info` ItemInfo))
  (bind _neckitem (`self.NeckItem`))
  (bind _primarylhanditem (`self.PrimaryLhandItem`))
  (bind _headitem (`self.HeadItem`))
  (bind _torsoitem (`self.TorsoItem`))
  (bind _leftarmitem (`self.LeftArmItem`))
  (bind _primaryrhanditem (`self.PrimaryRhandItem`))
  (bind _secondarylhanditem (`self.SecondaryLhandItem`))
  (bind _legsitem (`self.LegsItem`))
  (bind _feetitem (`self.FeetItem`))
  (bind _shielditem (`self.ShieldItem`))
  (bind _rightarmitem (`self.RightArmItem`))
  (bind _secondaryrhanditem (`self.SecondaryRhandItem`))
  (switch `/Game/++Enums/E_EquipmentSlots` _itemequipslot
    (:`NewEnumerator1`
      (`/Engine/EditorBlueprintResources/StandardMacros.IsValid` _headitem
        (:`Is Valid`
          (`self.K2_DestroyActor` _headitem))
        (:`Is Not Valid`
          _))
      (bind _returnvalue (`|SpawnActorFromClass` _itemclass (`self.GetTransform`) "AlwaysSpawn" "OverrideRootScale" null null))
      (bind _output_get (set `self.HeadItem` _returnvalue))
      (bind _asbase_armor_bp (cast `/Game/Interactables_BP/Armor/Base_Armor_BP` _output_get))
      (`self.K2_AttachToComponent` _asbase_armor_bp (`self.SkeletalMesh`) (`.MainAttachPoint_10_69C0D3114B0A7D89F6B55B9A2E8693E5` (break `/Game/++Structures/Armor_Info_S` (`/Game/Interactables_BP/Armor/Base_Armor_BP.ArmorInfo` _asbase_armor_bp))) "SnapToTarget" "SnapToTarget" "SnapToTarget" true)
      (`self.SetActorEnableCollision` _asbase_armor_bp false))
    (:`NewEnumerator2`
      (`/Engine/EditorBlueprintResources/StandardMacros.IsValid` _torsoitem
        (:`Is Valid`
          (`self.K2_DestroyActor` _torsoitem))
        (:`Is Not Valid`
          _))
      (bind _returnvalue_2 (`|SpawnActorFromClass` _itemclass (`self.GetTransform`) "AlwaysSpawn" "OverrideRootScale" null null))
      (bind _output_get_2 (set `self.TorsoItem` _returnvalue_2))
      (bind _asbase_armor_bp_2 (cast `/Game/Interactables_BP/Armor/Base_Armor_BP` _output_get_2))
      (`self.K2_AttachToComponent` _asbase_armor_bp_2 (`self.SkeletalMesh`) (`.MainAttachPoint_10_69C0D3114B0A7D89F6B55B9A2E8693E5` (break `/Game/++Structures/Armor_Info_S` (`/Game/Interactables_BP/Armor/Base_Armor_BP.ArmorInfo` _asbase_armor_bp_2))) "SnapToTarget" "SnapToTarget" "SnapToTarget" true)
      (`self.SetActorEnableCollision` _asbase_armor_bp_2 false))
    (:`NewEnumerator3`
      (`/Engine/EditorBlueprintResources/StandardMacros.IsValid` _rightarmitem
        (:`Is Valid`
          (`self.K2_DestroyActor` _rightarmitem))
        (:`Is Not Valid`
          _))
      (bind _returnvalue_3 (`|SpawnActorFromClass` _itemclass (`self.GetTransform`) "AlwaysSpawn" "OverrideRootScale" null null))
      (bind _output_get_3 (set `self.RightArmItem` _returnvalue_3))
      (bind _asbase_armor_bp_3 (cast `/Game/Interactables_BP/Armor/Base_Armor_BP` _output_get_3))
      (`self.K2_AttachToComponent` _asbase_armor_bp_3 (`self.SkeletalMesh`) (`.RightAttachPoint_11_4C5B8DC443D92F7385390CB8F5D6272E` (break `/Game/++Structures/Armor_Info_S` (`/Game/Interactables_BP/Armor/Base_Armor_BP.ArmorInfo` _asbase_armor_bp_3))) "SnapToTarget" "SnapToTarget" "SnapToTarget" true)
      (`self.SetActorEnableCollision` _asbase_armor_bp_3 false)
      (`/Engine/EditorBlueprintResources/StandardMacros.IsValid` _leftarmitem
        (:`Is Valid`
          (`self.K2_DestroyActor` _leftarmitem))
        (:`Is Not Valid`
          _))
      (bind _returnvalue_4 (`|SpawnActorFromClass` _itemclass (`self.GetTransform`) "AlwaysSpawn" "OverrideRootScale" null null))
      (bind _output_get_4 (set `self.LeftArmItem` _returnvalue_4))
      (bind _asbase_armor_bp_4 (cast `/Game/Interactables_BP/Armor/Base_Armor_BP` _output_get_4))
      (`self.K2_AttachToComponent` _asbase_armor_bp_4 (`self.SkeletalMesh`) (`.LeftAttachPoint_12_5F8469114C2708330A9F73B2EEE534F1` (break `/Game/++Structures/Armor_Info_S` (`/Game/Interactables_BP/Armor/Base_Armor_BP.ArmorInfo` _asbase_armor_bp_4))) "SnapToTarget" "SnapToTarget" "SnapToTarget" true)
      (`self.SetActorEnableCollision` _asbase_armor_bp_4 false))
    (:`NewEnumerator16`
      (`/Engine/EditorBlueprintResources/StandardMacros.IsValid` _shielditem
        (:`Is Valid`
          (`self.K2_DestroyActor` _shielditem))
        (:`Is Not Valid`
          _))
      (bind _returnvalue_5 (`|SpawnActorFromClass` _itemclass (`self.GetTransform`) "AlwaysSpawn" "OverrideRootScale" null null))
      (bind _output_get_5 (set `self.ShieldItem` _returnvalue_5))
      (bind _asbase_shield_bp (cast `/Game/Interactables_BP/Shields/Base_Shield_BP` _output_get_5))
      (`self.K2_AttachToComponent` _asbase_shield_bp (`self.SkeletalMesh`) (`.ShieldAttachPoint_5_E6F6811840D178EBB9FA2A8A2ED7E108` (break `/Game/++Structures/ShieldsInfo` (`/Game/Interactables_BP/Shields/Base_Shield_BP.ShieldInfo` _asbase_shield_bp))) "SnapToTarget" "SnapToTarget" "SnapToTarget" true)
      (`self.SetActorEnableCollision` _asbase_shield_bp false))
    (:`NewEnumerator4`
      (`/Engine/EditorBlueprintResources/StandardMacros.IsValid` _primaryrhanditem
        (:`Is Valid`
          (`self.K2_DestroyActor` _primaryrhanditem))
        (:`Is Not Valid`
          _))
      (bind _returnvalue_6 (`|SpawnActorFromClass` _itemclass (`self.GetTransform`) "AlwaysSpawn" "OverrideRootScale" null null))
      (bind _output_get_6 (set `self.PrimaryRhandItem` _returnvalue_6))
      (bind _asbase_weapons_bp (cast `/Game/Interactables_BP/Weapons/Base_Weapons_BP` _output_get_6))
      (`self.K2_AttachToComponent` _asbase_weapons_bp (`self.SkeletalMesh`) (`.PrimaryRightHand_13_66A281F448D463B37B8535AF5E7BD354` (break `/Game/++Structures/Weapons_Info_S` (`/Game/Interactables_BP/Weapons/Base_Weapons_BP.WeaponInfo` _asbase_weapons_bp))) "SnapToTarget" "SnapToTarget" "SnapToTarget" true)
      (`self.SetActorEnableCollision` _asbase_weapons_bp false))
    (:`NewEnumerator5`
      (`/Engine/EditorBlueprintResources/StandardMacros.IsValid` _primarylhanditem
        (:`Is Valid`
          (`self.K2_DestroyActor` _primarylhanditem))
        (:`Is Not Valid`
          _))
      (bind _returnvalue_7 (`|SpawnActorFromClass` _itemclass (`self.GetTransform`) "AlwaysSpawn" "OverrideRootScale" null null))
      (bind _output_get_7 (set `self.PrimaryLhandItem` _returnvalue_7))
      (bind _asbase_weapons_bp_2 (cast `/Game/Interactables_BP/Weapons/Base_Weapons_BP` _output_get_7))
      (`self.K2_AttachToComponent` _asbase_weapons_bp_2 (`self.SkeletalMesh`) (`.PrimaryLeftHand_15_B563D65C4EAE885BBFA4D58EA4CBCE46` (break `/Game/++Structures/Weapons_Info_S` (`/Game/Interactables_BP/Weapons/Base_Weapons_BP.WeaponInfo` _asbase_weapons_bp_2))) "SnapToTarget" "SnapToTarget" "SnapToTarget" true)
      (`self.SetActorEnableCollision` _asbase_weapons_bp_2 false))
    (:`NewEnumerator12`
      (`/Engine/EditorBlueprintResources/StandardMacros.IsValid` _secondaryrhanditem
        (:`Is Valid`
          (`self.K2_DestroyActor` _secondaryrhanditem))
        (:`Is Not Valid`
          _))
      (bind _returnvalue_8 (`|SpawnActorFromClass` _itemclass (`self.GetTransform`) "AlwaysSpawn" "OverrideRootScale" null null))
      (bind _output_get_8 (set `self.SecondaryRhandItem` _returnvalue_8))
      (bind _asbase_weapons_bp_3 (cast `/Game/Interactables_BP/Weapons/Base_Weapons_BP` _output_get_8))
      (`self.K2_AttachToComponent` _asbase_weapons_bp_3 (`self.SkeletalMesh`) (`.SecondaryRightHand_18_926F8CAD4C580FCD2C99D4883BD33467` (break `/Game/++Structures/Weapons_Info_S` (`/Game/Interactables_BP/Weapons/Base_Weapons_BP.WeaponInfo` _asbase_weapons_bp_3))) "SnapToTarget" "SnapToTarget" "SnapToTarget" true)
      (`self.SetActorEnableCollision` _asbase_weapons_bp_3 false))
    (:`NewEnumerator13`
      (`/Engine/EditorBlueprintResources/StandardMacros.IsValid` _secondarylhanditem
        (:`Is Valid`
          (`self.K2_DestroyActor` _secondarylhanditem))
        (:`Is Not Valid`
          _))
      (bind _returnvalue_9 (`|SpawnActorFromClass` _itemclass (`self.GetTransform`) "AlwaysSpawn" "OverrideRootScale" null null))
      (bind _output_get_9 (set `self.SecondaryLhandItem` _returnvalue_9))
      (bind _asbase_weapons_bp_4 (cast `/Game/Interactables_BP/Weapons/Base_Weapons_BP` _output_get_9))
      (`self.K2_AttachToComponent` _asbase_weapons_bp_4 (`self.SkeletalMesh`) (`.SecondaryLeftHand_19_A3179C2E40B396A57A8971A0801A8C84` (break `/Game/++Structures/Weapons_Info_S` (`/Game/Interactables_BP/Weapons/Base_Weapons_BP.WeaponInfo` _asbase_weapons_bp_4))) "SnapToTarget" "SnapToTarget" "SnapToTarget" true)
      (`self.SetActorEnableCollision` _asbase_weapons_bp_4 false))
    (:`NewEnumerator6`
      (`/Engine/EditorBlueprintResources/StandardMacros.IsValid` _legsitem
        (:`Is Valid`
          (`self.K2_DestroyActor` _legsitem))
        (:`Is Not Valid`
          _))
      (bind _returnvalue_10 (`|SpawnActorFromClass` _itemclass (`self.GetTransform`) "AlwaysSpawn" "OverrideRootScale" null null))
      (bind _output_get_10 (set `self.LegsItem` _returnvalue_10))
      (bind _asbase_armor_bp_5 (cast `/Game/Interactables_BP/Armor/Base_Armor_BP` _output_get_10))
      (`self.K2_AttachToComponent` _asbase_armor_bp_5 (`self.SkeletalMesh`) (`.MainAttachPoint_10_69C0D3114B0A7D89F6B55B9A2E8693E5` (break `/Game/++Structures/Armor_Info_S` (`/Game/Interactables_BP/Armor/Base_Armor_BP.ArmorInfo` _asbase_armor_bp_5))) "SnapToTarget" "SnapToTarget" "SnapToTarget" true)
      (`self.SetActorEnableCollision` _asbase_armor_bp_5 false))
    (:`NewEnumerator7`
      (`/Engine/EditorBlueprintResources/StandardMacros.IsValid` _feetitem
        (:`Is Valid`
          (`self.K2_DestroyActor` _feetitem))
        (:`Is Not Valid`
          _))
      (bind _returnvalue_11 (`|SpawnActorFromClass` _itemclass (`self.GetTransform`) "AlwaysSpawn" "OverrideRootScale" null null))
      (bind _output_get_11 (set `self.FeetItem` _returnvalue_11))
      (bind _asbase_armor_bp_6 (cast `/Game/Interactables_BP/Armor/Base_Armor_BP` _output_get_11))
      (`self.K2_AttachToComponent` _asbase_armor_bp_6 (`self.SkeletalMesh`) (`.MainAttachPoint_10_69C0D3114B0A7D89F6B55B9A2E8693E5` (break `/Game/++Structures/Armor_Info_S` (`/Game/Interactables_BP/Armor/Base_Armor_BP.ArmorInfo` _asbase_armor_bp_6))) "SnapToTarget" "SnapToTarget" "SnapToTarget" true)
      (`self.SetActorEnableCollision` _asbase_armor_bp_6 false))
    (:`NewEnumerator14`
      (`/Engine/EditorBlueprintResources/StandardMacros.IsValid` _neckitem
        (:`Is Valid`
          (`self.K2_DestroyActor` _neckitem))
        (:`Is Not Valid`
          _))
      (bind _returnvalue_12 (`|SpawnActorFromClass` _itemclass (`self.GetTransform`) "AlwaysSpawn" "OverrideRootScale" null null))
      (bind _output_get_12 (set `self.NeckItem` _returnvalue_12))
      (bind _asbase_amulette_bp (cast `/Game/Interactables_BP/Amulets/Base_Amulette_BP` _output_get_12))
      (`self.K2_AttachToComponent` _asbase_amulette_bp (`self.SkeletalMesh`) (`.AmuletAttachPoint_5_EB8D73994CCFF154ACFD84A8A5EADE1C` (break `/Game/++Structures/Amulet_Info` (`/Game/Interactables_BP/Amulets/Base_Amulette_BP.AmuletInfo` _asbase_amulette_bp))) "SnapToTarget" "SnapToTarget" "SnapToTarget" true)
      (`self.SetActorEnableCollision` _asbase_amulette_bp false))))

(fn `UnattachItem`
  (params (ItemInfo :type "/Game/++Structures/Item_Info Structure"))
  (switch `/Game/++Enums/E_EquipmentSlots` (`.ItemEquipSlot_21_E736EAB8438F0A6E85940E8CBD1C71C5` (break `/Game/++Structures/Item_Info` ItemInfo))
    (:`NewEnumerator1`
      (`self.K2_DestroyActor` (`self.HeadItem`)))
    (:`NewEnumerator2`
      (`self.K2_DestroyActor` (`self.TorsoItem`)))
    (:`NewEnumerator3`
      (`self.K2_DestroyActor` (`self.RightArmItem`))
      (`self.K2_DestroyActor` (`self.LeftArmItem`)))
    (:`NewEnumerator16`
      (`self.K2_DestroyActor` (`self.ShieldItem`)))
    (:`NewEnumerator4`
      (`self.K2_DestroyActor` (`self.PrimaryRhandItem`)))
    (:`NewEnumerator5`
      (`self.K2_DestroyActor` (`self.PrimaryLhandItem`)))
    (:`NewEnumerator12`
      (`self.K2_DestroyActor` (`self.SecondaryRhandItem`)))
    (:`NewEnumerator13`
      (`self.K2_DestroyActor` (`self.SecondaryLhandItem`)))
    (:`NewEnumerator6`
      (`self.K2_DestroyActor` (`self.LegsItem`)))
    (:`NewEnumerator7`
      (`self.K2_DestroyActor` (`self.FeetItem`)))
    (:`NewEnumerator14`
      (`self.K2_DestroyActor` (`self.NeckItem`)))))

(fn `UserConstructionScript`)